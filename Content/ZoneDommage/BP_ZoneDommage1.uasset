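; BP_ZoneDommage1 is a damage zone that hurts a BP_Phone actor entering its Box.
; Begin overlap casts to BP_Phone, sets InZone and starts a looping timer that applies fixed damage every second.
; The timer event clears itself only when InZone is false.
; End overlap sets InZone true again for a valid phone, so damage continues after it leaves the box.
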(event OnComponentBeginOverlap(Box)
  (params (OverlappedComponent :type Primitive%20Component%20Object%20Reference) (OtherActor :type Actor%20Object%20Reference) (OtherComp :type Primitive%20Component%20Object%20Reference) (OtherBodyIndex :type Integer) (bFromSweep :type Boolean) (SweepResult :type Hit%20Result%20Structure%20%28by%20ref%29))
  (bind _asbp_phone (Utilities|Casting|CastToBP_Phone OtherActor))
  (Utilities|IsValid _asbp_phone
    (:Is%20Valid
      (Variables|Default|SetInZone true)
      (if (Variables|Default|GetInZone)
        (bind _returnvalue (Utilities|Time|SetTimerbyEvent (delegate Custom|ApplyDamage) 1.0 true))))
    (:Is%20Not%20Valid
      (Variables|Default|SetInZone false))))

(event OnComponentEndOverlap(Box)
  (params (OverlappedComponent :type Primitive%20Component%20Object%20Reference) (OtherActor :type Actor%20Object%20Reference) (OtherComp :type Primitive%20Component%20Object%20Reference) (OtherBodyIndex :type Integer))
  (bind _asbp_phone (Utilities|Casting|CastToBP_Phone OtherActor))
  (Utilities|IsValid _asbp_phone
    (:Is%20Valid
      (Variables|Default|SetInZone true))
    (:Is%20Not%20Valid
      (Variables|Default|SetInZone false)
      (Development|PrintString "False"))))

(event Custom|ApplyDamage
  (Game|Damage|ApplyDamage (stale OnComponentBeginOverlap(Box) _asbp_phone) 8.0 0 0)
  (if (not (Variables|Default|GetInZone))
    (Utilities|Time|ClearandInvalidateTimerbyHandle (stale OnComponentBeginOverlap(Box) _returnvalue))))

(event EventBeginPlay)

(fn ConstructionScript)